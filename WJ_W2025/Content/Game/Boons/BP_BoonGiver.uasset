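; BP_BoonGiver generates random boon choices and applies a boon to a player.
; GenerateBoons constructs three objects from classes picked at random from PossibleBoon, with repeats possible, and returns them as SelectedBoons.
; AddBoon passes the given boon's Modifier to the player's ModifyStat.
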(event EventBeginPlay)

(fn GenerateBoons
  (while (< (LocalVariables|GetLoop) 3)
    (bind _returnvalue (Game|ConstructObjectfromClass (Utilities|Array|Get(acopy) (Variables|Default|GetPossibleBoon) (Math|Random|RandomInteger (Utilities|Array|Length (Variables|Default|GetPossibleBoon))))))
    (Utilities|Array|Add (LocalVariables|GetSelectedBoons) _returnvalue)
    (Math|Integer|IncrementInt (LocalVariables|GetLoop)))
  (return (LocalVariables|GetSelectedBoons)))

(fn AddBoon
  (params (Player :type BP%20Base%20Character%20Object%20Reference) (Boon :type BP%20Base%20Boon%20Object%20Reference))
  (Default|ModifyStat Player (Variables|/Game/Game/Boons/BP_BaseBoon.BP_BaseBoon_C|GetModifier Boon)))