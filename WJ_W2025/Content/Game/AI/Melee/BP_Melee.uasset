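; BP_Melee is a melee AI character child Blueprint that drives its Paper2D flipbook animations.
; On BeginPlay it runs the parent logic, sets the melee hit flipbook and binds to character movement updates.
; Movement updates switch to the walk flipbook when velocity is non-zero and back to idle when it stops.
; When playback finishes, attack and hit flipbooks return to idle, while any other flipbook restarts, acting as a manual loop.
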(event OnFinishedPlaying(PaperFlipbook)
  (bind _paperflipbook (Variables|Default|GetPaperFlipbook))
  (bind _returnvalue (Class|PaperFlipbookComponent|GetFlipbook _paperflipbook))
  (if (or (== _returnvalue "/Game/Game/AI/Melee/Spritesheet/Attack/FB_AttackMelee.FB_AttackMelee") (== _returnvalue "/Game/Game/AI/Melee/Spritesheet/Hit/FB_HitMelee.FB_HitMelee"))
    (Sprite|SetFlipbook (Variables|Default|GetPaperFlipbook) "/Game/Game/AI/Melee/Spritesheet/Idle/FB_IdleMelee.FB_IdleMelee")
    (else
      (Components|Timeline|PlayfromStart (Variables|Default|GetPaperFlipbook)))))

(event Custom|OnCharacterMovementUpdated_EventLich
  (params (DeltaSeconds :type Float%20%28single-precision%29) (OldLocation :type Vector) (OldVelocity :type Vector))
  (bind _paperflipbook (Variables|Default|GetPaperFlipbook))
  (bind _paperflipbook_2 (Variables|Default|GetPaperFlipbook))
  (if (Utilities|Operators|NotEqual(!=) :A (Transformation|GetVelocity))
    (if (not (== (Class|PaperFlipbookComponent|GetFlipbook _paperflipbook_2) "/Game/Game/AI/Melee/Spritesheet/Walk/FB_WalkMelee.FB_WalkMelee"))
      (Sprite|SetFlipbook _paperflipbook "/Game/Game/AI/Melee/Spritesheet/Walk/FB_WalkMelee.FB_WalkMelee")
      (Components|Timeline|PlayfromStart _paperflipbook))
    (elif (== (Class|PaperFlipbookComponent|GetFlipbook _paperflipbook_2) "/Game/Game/AI/Melee/Spritesheet/Walk/FB_WalkMelee.FB_WalkMelee")
      (Sprite|SetFlipbook _paperflipbook "/Game/Game/AI/Melee/Spritesheet/Idle/FB_IdleMelee.FB_IdleMelee"))))

(event EventBeginPlay
  (|CallParentFunction)
  (Variables|Default|SetHitFlipbook "/Game/Game/AI/Melee/Spritesheet/Hit/FB_HitMelee.FB_HitMelee")
  (EventDispatchers|AssignOnCharacterMovementUpdated (delegate Custom|OnCharacterMovementUpdated_EventLich)))

(fn ConstructionScript
  (|CallParentFunction))