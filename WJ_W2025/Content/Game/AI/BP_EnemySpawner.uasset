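; BP_EnemySpawner spawns enemies around its own location when play begins, using a map of enemy classes to counts.
; For each enemy, it picks a random reachable navmesh point within a fixed radius and re-rolls while that point is too close in 2D to any existing BP_BaseCharacter.
; Each spawned actor is then reported to BP_GameMode through OnEnemySpawn.
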(event EventBeginPlay
  (CallFunction|SpawnEnemy (Variables|Default|GetEnemyMap)))

(event Collision|EventActorBeginOverlap
  (params (OtherActor :type Actor%20Object%20Reference)))

(event EventTick
  (params (DeltaSeconds :type Float%20%28single-precision%29)))

(fn ConstructionScript)

(fn SpawnEnemy
  (params (Type :type Map%20of%20BP%20AI%20Base%20Class%20References%20to%20Integers))
  (bind _keys (Utilities|Map|Keys Type))
  (for _array_element _keys
    (for _index (range 1 (.Value (Utilities|Map|Find Type _array_element)))
      (bind _outactors (Actor|GetAllActorsOfClass "/Game/Game/Character/BP_BaseCharacter.BP_BaseCharacter_C"))
      (LocalVariables|SetrandomLoc (.RandomLocation (AI|Navigation|GetRandomReachablePointinRadius (Transformation|GetActorLocation) 2e+03 0 0)) :!label _label)
      (for _array_element_2 _outactors
        (if (< (Math|Vector|Distance2D(Vector) (LocalVariables|GetrandomLoc) (Transformation|GetActorLocation _array_element_2)) 5e+02)
          (goto _label)))
      (bind _returnvalue (Game|SpawnActorfromClass _array_element (Math|Transform|MakeTransform (LocalVariables|GetrandomLoc) "0, 0, 0" "1.000000,1.000000,1.000000") "Undefined" "MultiplyWithRoot" 0 0))
      (LocalVariables|SetrandomLoc "-999.000000,-999.000000,-999.000000")
      (bind _asbp_game_mode (Utilities|Casting|CastToBP_GameMode (Game|GetGameMode)))
      (Default|OnEnemySpawn _asbp_game_mode _returnvalue))))