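; BP_AIBase is a base enemy character using a Paper2D flipbook that takes hits and dies.
; Movement updates lock actor rotation to zero and face the sprite by flipping its X scale with velocity.
; Hit notifies the instigator, plays the hit flipbook and reduces health, then restores the previous flipbook or triggers death once.
; Death flags any archer controller, waits briefly, destroys the actor and notifies BP_GameMode.
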(event Custom|OnCharacterMovementUpdated_Event
  (params (DeltaSeconds :type Float%20%28single-precision%29) (OldLocation :type Vector) (OldVelocity :type Vector))
  (bind _paperflipbook (Variables|Default|GetPaperFlipbook))
  (Transformation|SetActorRotation "0, 0, 0")
  (if (and (Utilities|Operators|NotEqual(!=) :A (Transformation|GetVelocity)) (not (Variables|Default|GetisDying)))
    (if (> (.x (Transformation|GetVelocity)) 0.0)
      (Transformation|SetRelativeScale3D _paperflipbook "2.500000,1.000000,2.500000")
      (else
        (Transformation|SetRelativeScale3D _paperflipbook "-2.500000,1.000000,2.500000")))))

(event Custom|CharacterDeath
  (Variables|Default|SetisDying true)
  (bind _asbp_archer_controller (Utilities|Casting|CastToBP_ArcherController (Pawn|GetController))
    (:then
      (Default|SetIsDying _asbp_archer_controller))
    (:CastFailed
      _))
  (Utilities|FlowControl|Delay 1.5)
  (Actor|DestroyActor)
  (bind _asbp_game_mode (Utilities|Casting|CastToBP_GameMode (Game|GetGameMode)))
  (Default|OnEnemyDeath _asbp_game_mode self))

(event EventBeginPlay
  (EventDispatchers|AssignOnCharacterMovementUpdated (delegate Custom|OnCharacterMovementUpdated_Event))
  (Transformation|SetActorRotation "0, 0, 0")
  (Components|Timeline|SetLooping (Variables|Default|GetPaperFlipbook) false))

(event Collision|EventActorBeginOverlap
  (params (OtherActor :type Actor%20Object%20Reference)))

(event EventHit
  (params (Instigator :type Actor%20Object%20Reference) (Damage :type Float%20%28double-precision%29))
  (bind _paperflipbook (Variables|Default|GetPaperFlipbook))
  (bind _returnvalue (Class|PaperFlipbookComponent|GetFlipbook _paperflipbook))
  (if (not (Variables|Default|GetisDying))
    (Class|IHittable|HitReturn(Message) Instigator)
    (if (!= _returnvalue (Variables|Default|GetHitFlipbook))
      (Variables|Default|SetPreviousFlipbook _returnvalue))
    (Sprite|SetFlipbook _paperflipbook (Variables|Default|GetHitFlipbook))
    (Components|Timeline|PlayfromStart _paperflipbook)
    (Variables|Default|SetHealth (- (Variables|Default|GetHealth) Damage))
    (if (<= (Variables|Default|GetHealth) 0.0)
      (Utilities|FlowControl|DoOnce false
        (:Completed
          (CallFunction|CharacterDeath)))
      (else
        (Utilities|FlowControl|Delay (Class|PaperFlipbookComponent|GetFlipbookLength _paperflipbook))
        (Sprite|SetFlipbook _paperflipbook (Variables|Default|GetPreviousFlipbook))))))

(fn ConstructionScript)