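; Game mode that runs a level as one enemy wave in a boon-based run, handling victory and game over.
; BeginPlay totals the wave's enemies from DT_Waves using the GameInstance's progress and binds every player's death, showing Game Over once all die.
; Clearing the wave opens boon selection; the pick advances progress, saves boon and player resources, then opens a random level, rerolled to differ from the current one.
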(event Custom|OnEnemySpawn
  (params (EnemySpawned :type BP%20AI%20Base%20Object%20Reference))
  (bind _returnvalue (Utilities|GetClass EnemySpawned))
  (bind _currentenemies (Variables|Default|GetCurrentEnemies))
  (if (Utilities|Map|Contains _currentenemies _returnvalue)
    (Utilities|Map|Add _currentenemies _returnvalue (+ (.Value (Utilities|Map|Find _currentenemies _returnvalue)) 1))
    (else
      (Utilities|Map|Add _currentenemies _returnvalue 1))))

(event Custom|OnEnemyDeath
  (params (EnemyDeath :type BP%20AI%20Base%20Object%20Reference))
  (Math|Integer|DecrementInt (Variables|Default|GetEnemyInWave)
    (:%20%20
      (if (<= (Variables|Default|GetEnemyInWave) 0)
        (CallFunction|SelectBoon)))))

(event Custom|PlayerSelectedBoon
  (params (Boon :type BP%20Base%20Boon%20Object%20Reference) (PlayerIndex :type Integer))
  (bind _asbp_game_instance (Utilities|Casting|CastToBP_GameInstance (Game|GetGameInstance)))
  (bind _result (Math|Integer|IncrementInt (Variables|/Game/Game/GameSettings/BP_GameInstance.BP_GameInstance_C|GetCurrentProgress _asbp_game_instance))
    (:%20%20
      (Variables|/Game/Game/GameSettings/BP_GameInstance.BP_GameInstance_C|SetCurrentProgress _asbp_game_instance _result)
      (Default|SaveBoon _asbp_game_instance PlayerIndex Boon)
      (CallFunction|SaveRess)
      (bind _outmap (CallFunction|SelectRandomLevel))
      (Game|OpenLevel(byObjectReference) (Utilities|Struct|BreakSoftWorldReference _outmap)))))

(event Custom|PlayerDeath
  (params (PlayerID :type Integer))
  (Utilities|Array|Add (Variables|Default|GetPlayerDiedId) PlayerID)
  (if (>= (Utilities|Array|Length (Variables|Default|GetPlayerDiedId)) (Variables|Default|GetPlayersNumb))
    (CallFunction|GameOver)))

(event EventBeginPlay
  (bind _asbp_game_instance (Utilities|Casting|CastToBP_GameInstance (Game|GetGameInstance))
    (:then
      (bind _returnvalue (Utilities|GetDataTableRow "/Game/Game/GameSettings/DT_Waves.DT_Waves" (Utilities|String|StringToName (Utilities|String|ToString(Integer) (Variables|/Game/Game/GameSettings/BP_GameInstance.BP_GameInstance_C|GetCurrentProgress _asbp_game_instance))))
        (:then
          (bind _keys (Utilities|Map|Keys (.EnemyMap (Utilities|Struct|BreakS_WavesInfo _returnvalue))))
          (for _array_element _keys
            (Variables|Default|SetEnemyInWave (+ (.Value (Utilities|Map|Find (.EnemyMap (Utilities|Struct|BreakS_WavesInfo _returnvalue)) _array_element)) (Variables|Default|GetEnemyInWave)))))))
    (:CastFailed
      _))
  (bind _outactors (Actor|GetAllActorsOfClass "/Game/Game/Character/BP_BaseCharacter.BP_BaseCharacter_C"))
  (for _array_element_2 _outactors
    (EventDispatchers|BindEventtoOnPlayerDeath _array_element_2 (delegate Custom|PlayerDeath))
    (bind _result (Math|Integer|IncrementInt (Variables|Default|GetPlayersNumb))
      (:%20%20
        (Variables|Default|SetPlayersNumb _result)))))

(fn ConstructionScript)

(fn SelectRandomLevel
  (bind _returnvalue (Game|GetCurrentLevelName true))
  (switch string _returnvalue
    (:Default
      (LocalVariables|SetWorldAsset "/Game/Game/Levels/MainMenu.MainMenu"))
    (:GameLevel_CityInBackground
      (LocalVariables|SetWorldAsset "/Game/Game/Levels/GameLevel_CityInBackground.GameLevel_CityInBackground"))
    (:GameLevel_Cityscape
      (LocalVariables|SetWorldAsset "/Game/Game/Levels/GameLevel_Cityscape.GameLevel_Cityscape"))
    (:GameLevel_Mountains
      (LocalVariables|SetWorldAsset "/Game/Game/Levels/GameLevel_Mountains.GameLevel_Mountains")))
  (LocalVariables|SetrandomLevel (.OutItem (Utilities|Array|Random (LocalVariables|GetPossibleLevels))) :!label _label)
  (if (== (Utilities|Struct|BreakSoftWorldReference (LocalVariables|GetrandomLevel)) (Utilities|Struct|BreakSoftWorldReference (Utilities|Struct|MakeSoftWorldReference (LocalVariables|GetWorldAsset))))
    (goto _label)
    (else
      (Variables|Default|SetCurrentLevel (LocalVariables|GetrandomLevel))
      (return (LocalVariables|GetrandomLevel)))))

(fn SelectBoon
  (bind _returnvalue (Game|GetPlayerController 0))
  (bind _boons (Default|GenerateBoons (Variables|Default|GetBP_BoonGiver)))
  (bind _returnvalue_2 (UserInterface|CreateWidget "/Game/Game/Boons/UI/WBP_BoonSelection.WBP_BoonSelection_C" _returnvalue _boons))
  (EventDispatchers|BindEventtoOnBoonSelected _returnvalue_2 (EventDispatchers|CreateEvent :!event Custom|PlayerSelectedBoon))
  (UserInterface|Viewport|AddtoViewport _returnvalue_2 0)
  (Input|SetInputModeUIOnly _returnvalue _returnvalue_2 "DoNotLock" false)
  (Variables|/Script/Engine.PlayerController|SetbShowMouseCursor _returnvalue true))

(fn SaveRess
  (bind _asbp_game_instance (Utilities|Casting|CastToBP_GameInstance (Game|GetGameInstance)))
  (bind _outactors (Actor|GetAllActorsOfClass "/Game/Game/Character/BP_BaseCharacter.BP_BaseCharacter_C"))
  (for _array_element _outactors
    (bind _asplayer_controller (Utilities|Casting|CastToPlayerController (Pawn|GetController _array_element)))
    (Default|SaveRessources _asbp_game_instance (Variables|/Game/Game/Character/BP_BaseCharacter.BP_BaseCharacter_C|GetHealth _array_element) (Variables|/Game/Game/Character/BP_BaseCharacter.BP_BaseCharacter_C|GetPotentialLife _array_element) (Class|GameplayStatics|GetPlayerControllerID _asplayer_controller))))

(fn GameOver
  (bind _returnvalue (Game|GetPlayerController 0))
  (bind _returnvalue_2 (UserInterface|CreateWidget "/Game/Game/Widget/WBP_GameOver.WBP_GameOver_C" _returnvalue))
  (UserInterface|Viewport|AddtoViewport _returnvalue_2 0)
  (Input|SetInputModeUIOnly _returnvalue 0 "DoNotLock" false)
  (Variables|/Script/Engine.PlayerController|SetbShowMouseCursor _returnvalue true))