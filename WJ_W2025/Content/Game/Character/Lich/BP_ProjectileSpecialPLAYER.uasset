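; Player Lich special-attack projectile whose speed, damage and blast size come from its Stats.
; It flips its flipbook to match travel direction, then after a short lifetime either explodes (with AoE) or is destroyed.
; Overlapping an I_Hittable other than BP_BaseCharacter deals damage, explodes with AoE, and plays a scaled impact flipbook before destruction.
; Explode uses a sphere trace to damage BP_AIBase actors.
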(event OnComponentBeginOverlap(Collision)
  (params (OverlappedComponent :type Primitive%20Component%20Object%20Reference) (OtherActor :type Actor%20Object%20Reference) (OtherComp :type Primitive%20Component%20Object%20Reference) (OtherBodyIndex :type Integer) (bFromSweep :type Boolean) (SweepResult :type Hit%20Result%20Structure%20%28by%20ref%29))
  (bind _stats (Variables|Default|GetStats))
  (bind _paperflipbook (Variables|Default|GetPaperFlipbook))
  (bind _relativescale3d (Variables|/Script/Engine.SceneComponent|GetRelativeScale3D _paperflipbook))
  (Utilities|Casting|CastToBP_BaseCharacter OtherActor
    (:CastFailed
      (if (Utilities|DoesObjectImplementInterface OtherActor "/Game/Game/Interface/I_Hittable.I_Hittable_C")
        (Class|IHittable|Hit(Message) OtherActor (Variables|Actor|GetInstigator) (* (Variables|Default|GetBaseDamage) (.attack _stats)))
        (Variables|/Script/Engine.PrimitiveComponent|SetbGenerateOverlapEvents (Variables|Default|GetCollision) false)
        (if (> (.aoe _stats) 0.0)
          (CallFunction|Explode)
          (Variables|/Script/Engine.MovementComponent|SetVelocity (Variables|Default|GetProjectileMovement) "0, 0, 0"))
        (Sprite|SetFlipbook _paperflipbook "/Game/Game/Character/Lich/Spritesheet/ProjectileSkill/FB_SkillImpactLich.FB_SkillImpactLich")
        (Transformation|SetWorldScale3D _paperflipbook (Math|Vector|MakeVector (* (.x _relativescale3d) (.aoe _stats)) 1.0 (* (.z _relativescale3d) (.aoe _stats))))
        (Utilities|FlowControl|Delay (Class|PaperFlipbookComponent|GetFlipbookLength _paperflipbook))
        (Actor|DestroyActor)))))

(event EventBeginPlay
  (bind _returnvalue (Transformation|GetActorRotation))
  (bind _paperflipbook (Variables|Default|GetPaperFlipbook))
  (Audio|PlaySound2D "/Game/Game/SFX/ProjectileShoot.ProjectileShoot" 1.0 1.0 0.0 0 0)
  (if (== (Math|Float|Sign(Float) (.x (Transformation|GetVelocity))) 1.0)
    (Transformation|SetWorldRotation _paperflipbook (Math|Rotator|MakeRotator (.roll _returnvalue) (.pitch _returnvalue) 0.0) false false)
    (else
      (Transformation|SetWorldRotation _paperflipbook (Math|Rotator|MakeRotator (.roll _returnvalue) (.pitch _returnvalue) 1.8e+02) false false)))
  (Utilities|FlowControl|Delay 2.0)
  (if (> (.aoe (Variables|Default|GetStats)) 0.0)
    (CallFunction|Explode)
    (else
      (Actor|DestroyActor))))

(event Collision|EventActorBeginOverlap
  (params (OtherActor :type Actor%20Object%20Reference)))

(event EventTick
  (params (DeltaSeconds :type Float%20%28single-precision%29)))

(fn ConstructionScript
  (bind _stats (Variables|Default|GetStats))
  (bind _projectilemovement (Variables|Default|GetProjectileMovement))
  (Variables|/Script/Engine.ProjectileMovementComponent|SetInitialSpeed _projectilemovement (.speed _stats))
  (Variables|/Script/Engine.ProjectileMovementComponent|SetMaxSpeed _projectilemovement (.speed _stats)))

(fn Explode
  (bind _returnvalue (Transformation|GetActorLocation))
  (bind _stats (Variables|Default|GetStats))
  (Audio|PlaySound2D "/Game/Game/SFX/LichSkillImpact.LichSkillImpact" 1.0 1.0 0.0 0 0)
  (bind (_outhits _returnvalue_2) (Collision|MultiSphereTraceByChannel _returnvalue _returnvalue (* (Variables|Default|GetBaseAoE) (.aoe _stats)) "TraceTypeQuery2" false 0 "None" true "(R=1.000000,G=0.000000,B=0.000000,A=0.000000)" "(R=0.000000,G=1.000000,B=0.000000,A=0.000000)" 0.0))
  (if _returnvalue_2
    (for _array_element _outhits
      (bind _asbp_aibase (Utilities|Casting|CastToBP_AIBase (.hitactor _array_element)))
      (Class|IHittable|Hit(Message) _asbp_aibase (Variables|Actor|GetInstigator) (* (Variables|Default|GetBaseDamage) (.attack _stats))))))