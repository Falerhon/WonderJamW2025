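; BP_Projectile is a projectile in the Lich character's folder that damages hittable actors it overlaps.
; The construction script sets the ProjectileMovement initial and max speed from Stats.
; Collision overlaps ignore the instigator and send I_Hittable actors a HitMessage with base damage scaled by the Attack stat, then destroy the projectile.
; Other overlaps leave it flying, and a short BeginPlay delay limits its lifetime.
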(event OnComponentBeginOverlap(Collision)
  (params (OverlappedComponent :type Primitive%20Component%20Object%20Reference) (OtherActor :type Actor%20Object%20Reference) (OtherComp :type Primitive%20Component%20Object%20Reference) (OtherBodyIndex :type Integer) (bFromSweep :type Boolean) (SweepResult :type Hit%20Result%20Structure%20%28by%20ref%29))
  (if (!= OtherActor (Game|GetInstigator))
    (if (Utilities|DoesObjectImplementInterface OtherActor "/Game/Game/Interface/I_Hittable.I_Hittable_C")
      (Class|IHittable|Hit(Message) OtherActor (Variables|Actor|GetInstigator) (* (Variables|Default|GetBaseDamage) (.attack (Variables|Default|GetStats))))
      (Actor|DestroyActor))))

(event EventBeginPlay
  (Utilities|FlowControl|Delay 2.0)
  (Actor|DestroyActor))

(event Collision|EventActorBeginOverlap
  (params (OtherActor :type Actor%20Object%20Reference)))

(event EventTick
  (params (DeltaSeconds :type Float%20%28single-precision%29)))

(fn ConstructionScript
  (bind _stats (Variables|Default|GetStats))
  (bind _projectilemovement (Variables|Default|GetProjectileMovement))
  (Variables|/Script/Engine.ProjectileMovementComponent|SetInitialSpeed _projectilemovement (.speed _stats))
  (Variables|/Script/Engine.ProjectileMovementComponent|SetMaxSpeed _projectilemovement (.speed _stats)))