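; BP_MeleeAttack is a short-lived melee hit actor for the Schrodinger character, pairing a Paper2D flipbook effect with a Box overlap volume.
; On spawn it resets the flipbook's world yaw to zero, then destroys itself once the animation's length elapses.
; Box overlaps with non-instigator actors implementing I_Hittable send a HitMessage with base damage scaled by the Attack stat.
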(event OnComponentBeginOverlap(Box)
  (params (OverlappedComponent :type Primitive%20Component%20Object%20Reference) (OtherActor :type Actor%20Object%20Reference) (OtherComp :type Primitive%20Component%20Object%20Reference) (OtherBodyIndex :type Integer) (bFromSweep :type Boolean) (SweepResult :type Hit%20Result%20Structure%20%28by%20ref%29))
  (if (!= OtherActor (Game|GetInstigator))
    (if (Utilities|DoesObjectImplementInterface OtherActor "/Game/Game/Interface/I_Hittable.I_Hittable_C")
      (Class|IHittable|Hit(Message) OtherActor (Variables|Actor|GetInstigator) (* (Variables|Default|GetBaseDamage) (.attack (Variables|Default|GetStats)))))))

(event EventBeginPlay
  (bind _returnvalue (Transformation|GetActorRotation))
  (Transformation|SetWorldRotation (Variables|Default|GetPaperFlipbook) (Math|Rotator|MakeRotator (.roll _returnvalue) (.pitch _returnvalue) 0.0) false false)
  (Utilities|FlowControl|Delay (Class|PaperFlipbookComponent|GetFlipbookLength (Variables|Default|GetPaperFlipbook)))
  (Actor|DestroyActor))

(event Collision|EventActorBeginOverlap
  (params (OtherActor :type Actor%20Object%20Reference)))

(fn ConstructionScript)