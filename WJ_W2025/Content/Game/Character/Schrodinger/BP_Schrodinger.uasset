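; Schrodinger character Blueprint, a child class that drives flipbook animation and spawns the character's attack and special ability actors.
; Movement updates switch between walk and idle flipbooks; finished attack or skill animations return to idle, while others replay.
; Attack, when targeted, spawns an aimed actor offset toward the target point.
; Special, once PaySpecial succeeds, spawns an AoE-scaled actor at the character's XY, passing stats derived from CurrentStats.
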(event OnFinishedPlaying(PaperFlipbook)
  (bind _paperflipbook (Variables|Default|GetPaperFlipbook))
  (bind _returnvalue (Class|PaperFlipbookComponent|GetFlipbook _paperflipbook))
  (if (or (== _returnvalue "/Game/Game/Character/Schrodinger/Spritesheet/Attack/FB_AttackSchrodinger.FB_AttackSchrodinger") (== _returnvalue "/Game/Game/Character/Schrodinger/Spritesheet/Skill/FB_SkillSchroddinger.FB_SkillSchroddinger"))
    (Sprite|SetFlipbook (Variables|Default|GetPaperFlipbook) "/Game/Game/Character/Schrodinger/Spritesheet/Idle/FB_IdleSchrodinger.FB_IdleSchrodinger")
    (else
      (Components|Timeline|PlayfromStart (Variables|Default|GetPaperFlipbook)))))

(event Custom|OnCharacterMovementUpdated_EventSchrodinger
  (params (DeltaSeconds :type Float%20%28single-precision%29) (OldLocation :type Vector) (OldVelocity :type Vector))
  (bind _paperflipbook (Variables|Default|GetPaperFlipbook))
  (bind _paperflipbook_2 (Variables|Default|GetPaperFlipbook))
  (if (Utilities|Operators|NotEqual(!=) :A (Transformation|GetVelocity))
    (if (not (== (Class|PaperFlipbookComponent|GetFlipbook (Variables|Default|GetPaperFlipbook)) "/Game/Game/Character/Schrodinger/Spritesheet/Walk/FB_WalkSchrodinger.FB_WalkSchrodinger"))
      (Sprite|SetFlipbook _paperflipbook "/Game/Game/Character/Schrodinger/Spritesheet/Walk/FB_WalkSchrodinger.FB_WalkSchrodinger")
      (Components|Timeline|PlayfromStart _paperflipbook))
    (elif (== (Class|PaperFlipbookComponent|GetFlipbook _paperflipbook_2) "/Game/Game/Character/Schrodinger/Spritesheet/Walk/FB_WalkSchrodinger.FB_WalkSchrodinger")
      (Sprite|SetFlipbook _paperflipbook_2 "/Game/Game/Character/Schrodinger/Spritesheet/Idle/FB_IdleSchrodinger.FB_IdleSchrodinger"))))

(event EventBeginPlay
  (|CallParentFunction)
  (EventDispatchers|AssignOnCharacterMovementUpdated (delegate Custom|OnCharacterMovementUpdated_EventSchrodinger)))

(event Collision|EventActorBeginOverlap
  (params (OtherActor :type Actor%20Object%20Reference)))

(event EventTick
  (params (DeltaSeconds :type Float%20%28single-precision%29)))

(fn ConstructionScript
  (|CallParentFunction))

(fn Attack
  (params (Location :type Vector :default "0, 0, 0") (Targeted :type Boolean))
  (bind _returnvalue (Transformation|GetActorLocation))
  (bind _paperflipbook (Variables|Default|GetPaperFlipbook))
  (bind _capsulecomponent (Variables|Default|GetCapsuleComponent))
  (bind _returnvalue_2 (Components|Capsule|GetScaledCapsuleHalfHeight _capsulecomponent))
  (bind _returnvalue_3 (Math|Vector|MakeVector (.x Location) (.y Location) _returnvalue_2))
  (if Targeted
    (Sprite|SetFlipbook _paperflipbook "/Game/Game/Character/Schrodinger/Spritesheet/Attack/FB_AttackSchrodinger.FB_AttackSchrodinger")
    (Components|Timeline|PlayfromStart _paperflipbook)
    (Game|SpawnActorfromClass (Variables|Default|GetAttackClass) (Math|Transform|MakeTransform (+ _returnvalue (* (Math|Vector|GetUnitDirection(Vector) _returnvalue _returnvalue_3) (Variables|Default|GetAttackSpawnDistance))) (Math|Rotator|FindLookatRotation _returnvalue _returnvalue_3)) "Undefined" "MultiplyWithRoot" 0 (Utilities|Struct|MakeS_AbilityStats (.attack (CallFunction|CurrentStats)) 1.2e+03 0.0) self)))

(fn Special
  (params (Location :type Vector :default "0, 0, 0") (Targeted :type Boolean))
  (bind _stats (CallFunction|CurrentStats))
  (bind _returnvalue (Transformation|GetActorTransform))
  (bind _paperflipbook (Variables|Default|GetPaperFlipbook))
  (LocalVariables|SetTargetLocation Location)
  (bind _couldpay (CallFunction|PaySpecial))
  (if _couldpay
    (Sprite|SetFlipbook _paperflipbook "/Game/Game/Character/Schrodinger/Spritesheet/Skill/FB_SkillSchroddinger.FB_SkillSchroddinger")
    (Components|Timeline|PlayfromStart _paperflipbook)
    (Game|SpawnActorfromClass (Variables|Default|GetSpecialClass) (Math|Transform|MakeTransform (Math|Vector|MakeVector (.x (.location _returnvalue)) (.y (.location _returnvalue)) (* 52.0 (.specialaoe _stats)))) "Undefined" "MultiplyWithRoot" 0 (Utilities|Struct|MakeS_AbilityStats (+ (.attack _stats) (.specialattscale _stats)) 1.5e+03 (.specialaoe _stats)) self)
    (else
      (return))))