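; Base 2D flipbook player character that switches between Alive and Undead states as Health crosses a threshold, each with its own stats.
; Landed hits build PotentialLife, which pays for healing; PaySpecial charges Health when Alive, PotentialLife when Undead.
; Attack and Special inputs query EQS for the closest enemy, then call placeholder functions.
; BeginPlay restores saved resources and boons from the game instance, applying stat modifiers per state or to both.
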(event Custom|TriggerSpecial
  (params (QueryInstance :type Env%20Query%20Instance%20Blueprint%20Wrapper%20Object%20Reference) (QueryStatus :type EEnvQueryStatus%20Enum :default "Processing"))
  ;[1 1 1] Special
  (bind (_resultlocations _returnvalue) (AI|EQS|GetQueryResultsasLocations QueryInstance))
  (CallFunction|Special (Utilities|Array|Get(acopy) _resultlocations) _returnvalue))

(event Custom|TriggerAttack
  (params (QueryInstance :type Env%20Query%20Instance%20Blueprint%20Wrapper%20Object%20Reference) (QueryStatus :type EEnvQueryStatus%20Enum :default "Processing"))
  ;[1 1 1] Attack
  (bind (_resultlocations _returnvalue) (AI|EQS|GetQueryResultsasLocations QueryInstance))
  (CallFunction|Attack (Utilities|Array|Get(acopy) _resultlocations) _returnvalue))

(event Custom|OnCharacterMovementUpdated_Event
  (params (DeltaSeconds :type Float%20%28single-precision%29) (OldLocation :type Vector) (OldVelocity :type Vector))
  (bind _paperflipbook (Variables|Default|GetPaperFlipbook))
  (if (Utilities|Operators|NotEqual(!=) :A (Transformation|GetVelocity))
    (Transformation|SetActorRotation "0, 0, 0")
    (if (> (.x (Transformation|GetVelocity)) 0.0)
      (Transformation|SetRelativeScale3D _paperflipbook "2.500000,1.000000,2.500000")
      (else
        (Transformation|SetRelativeScale3D _paperflipbook "-2.500000,1.000000,2.500000")))))

(event Input|EnhancedActionEvents|EnhancedInputActionIA_Move
  (params (ActionValue :type Vector%202D%20Structure) (ElapsedSeconds :type Float%20%28double-precision%29) (TriggeredSeconds :type Float%20%28double-precision%29) (InputAction :type Input%20Action%20Object%20Reference :default "/Game/ThirdPerson/Input/Actions/IA_Move.IA_Move"))
  (bind _returnvalue (Pawn|GetControlRotation :!class /Script/Engine.Pawn))
  ;[1 1 1] Movement
  (Pawn|Input|AddMovementInput (Math|Vector|GetRightVector (Math|Rotator|MakeRotator (.roll _returnvalue) 0.0 (.yaw _returnvalue))) (.x ActionValue) false)
  (Pawn|Input|AddMovementInput (Math|Vector|GetForwardVector (Math|Rotator|MakeRotator 0.0 0.0 (.yaw (Pawn|GetControlRotation :!class /Script/Engine.Pawn)))) (.y ActionValue) false))

(event Input|EnhancedActionEvents|EnhancedInputActionIA_Attack
  (params (ActionValue :type Boolean) (ElapsedSeconds :type Float%20%28double-precision%29) (TriggeredSeconds :type Float%20%28double-precision%29) (InputAction :type Input%20Action%20Object%20Reference :default "/Game/Game/Character/Controlls/Actions/IA_Attack.IA_Attack"))
  ;[1 1 1] Attack
  (bind _returnvalue (AI|EQS|RunEQSQuery "/Game/Game/Character/EQS_FindClosestEnemy.EQS_FindClosestEnemy" self "SingleResult"))
  (EventDispatchers|BindEventtoOnQueryFinishedEvent _returnvalue (delegate Custom|TriggerAttack)))

(event Input|EnhancedActionEvents|EnhancedInputActionIA_Heal
  (params (ActionValue :type Boolean) (ElapsedSeconds :type Float%20%28double-precision%29) (TriggeredSeconds :type Float%20%28double-precision%29) (InputAction :type Input%20Action%20Object%20Reference :default "/Game/Game/Character/Controlls/Actions/IA_Heal.IA_Heal"))
  ;[1 1 1] Heal
  (CallFunction|Heal))

(event Input|EnhancedActionEvents|EnhancedInputActionIA_Special
  (params (ActionValue :type Boolean) (ElapsedSeconds :type Float%20%28double-precision%29) (TriggeredSeconds :type Float%20%28double-precision%29) (InputAction :type Input%20Action%20Object%20Reference :default "/Game/Game/Character/Controlls/Actions/IA_Special.IA_Special"))
  ;[1 1 1] Special
  (bind _returnvalue (AI|EQS|RunEQSQuery "/Game/Game/Character/EQS_FindClosestEnemy.EQS_FindClosestEnemy" self "SingleResult"))
  (EventDispatchers|BindEventtoOnQueryFinishedEvent _returnvalue (delegate Custom|TriggerSpecial)))

(event EventHit
  (params (Instigator :type Actor%20Object%20Reference) (Damage :type Float%20%28double-precision%29))
  ;[1 1 1] Getting hit
  (Development|PrintString (Utilities|String|Append (Utilities|GetDisplayName Instigator) " HIT ME") true true "(R=1.000000,G=0.000000,B=0.063341,A=1.000000)"))

(event EventBeginPlay
  ;[1 1 1] InputMapping
  (CallFunction|LoadStatsfromGameInstance)
  (bind _asplayer_controller (Utilities|Casting|CastToPlayerController (Pawn|GetController)))
  (Utilities|IsValid (PlayerController|LocalPlayerSubsystems|GetEnhancedInputLocalPlayerSubsystem _asplayer_controller)
    (:Is%20Valid
      (Input|AddMappingContext (PlayerController|LocalPlayerSubsystems|GetEnhancedInputLocalPlayerSubsystem _asplayer_controller) "/Game/Game/Character/Controlls/IMC_Player.IMC_Player" 0 "(bIgnoreAllPressedKeysUntilRelease=True,bForceImmediately=False,bNotifyUserSettings=False)")
      (Character|BindEventtoOnCharacterMovementUpdated (delegate Custom|OnCharacterMovementUpdated_Event))
      (Components|Timeline|SetLooping (Variables|Default|GetPaperFlipbook) false)
      (Transformation|SetActorRotation "0, 0, 0"))))

(event EventHitReturn
  (CallFunction|ModifyPotentialLife (* (Variables|Default|GetBasePotentialLifeRegen) (.potentialliferegenrate (CallFunction|CurrentStats)))))

(event Input|KeyboardEvents|Q
  (params (Key :type Key%20Structure :default "None"))
  ;[1 1 1] Test self damage
  (:Pressed
    (CallFunction|ModifyHealth -1e+01)))

(fn ConstructionScript)

(fn Attack
  (params (Location :type Vector) (Targeted :type Boolean))
  (Development|PrintString "Attacking"))

(fn Special
  (params (Location :type Vector) (Targeted :type Boolean)))

(fn Heal
  (if (>= (Variables|Default|GetPotentialLife) (.healcost (CallFunction|CurrentStats)))
    (CallFunction|ModifyPotentialLife -25.0)
    (CallFunction|ModifyHealth 5.0)))

(fn CurrentStats
  (return (.Value (Utilities|Map|Find (Variables|Default|GetStats) (Variables|Default|GetCurrentState)))))

(fn ModifyStat
  (params (Modification :type S%20Modifiers%20Structure))
  (if (Utilities|Enum|NotEqual(Enum) (.state Modification) "NewEnumerator2")
    (|StatedModification (.affectedstat Modification) (.type Modification) (.modifier Modification) (.state Modification))
    (else
      (|GlobalStatModification (.type Modification) (.modifier Modification) (.affectedstat Modification)))))

(fn GetStat
  (params (Stat :type E_CharacterStats%20Enum :default "NewEnumerator0"))
  (bind _stats (CallFunction|CurrentStats))
  (switch Utilities|FlowControl|Switch|SwitchonE_CharacterStats Stat
    (:NewEnumerator0
      (return (.attack _stats)))
    (:NewEnumerator1
      (return (.attackspeed _stats)))
    (:NewEnumerator2
      (return 0.0))
    (:NewEnumerator3
      (return (.maxpotentiallife _stats)))
    (:NewEnumerator4
      (return (Variables|Default|GetHealth)))
    (:NewEnumerator5
      (return (.maxhealth _stats)))
    (:NewEnumerator6
      (return (.minhealth _stats)))
    (:NewEnumerator7
      (return (Variables|Default|GetUndeadThreshold)))))

(fn ApplyModification
  (params (Stat :type Float%20%28double-precision%29%20%28by%20ref%29) (Type :type E_Modificator%20Enum :default "NewEnumerator0") (Modification :type Float%20%28double-precision%29))
  (switch Utilities|FlowControl|Switch|SwitchonE_Modificator Type
    (:NewEnumerator0
      (|SetBy-RefVar Stat (Math|Float|Clamp(Float) (+ Stat (* Stat Modification)) 0.0 1e+04)))
    (:NewEnumerator1
      (|SetBy-RefVar Stat (+ Stat Modification)))
    (:NewEnumerator2
      (|SetBy-RefVar Stat (Math|Float|Clamp(Float) (- Stat Modification) 0.0 1e+04)))))

(fn ModifyPotentialLife
  (params (Modification :type Float%20%28double-precision%29))
  (bind _stats (CallFunction|CurrentStats))
  (if (< (+ (Variables|Default|GetPotentialLife) Modification) (.maxpotentiallife _stats))
    (Variables|Default|SetPotentialLife (+ (Variables|Default|GetPotentialLife) Modification))
    (elif (> (+ (Variables|Default|GetPotentialLife) Modification) 0.0)
      (Variables|Default|SetPotentialLife (.maxpotentiallife _stats))
      (else
        (Variables|Default|SetPotentialLife 0.0))))
  (Development|PrintString (Utilities|String|Append "Cuurent Potential : " (Utilities|String|ToString(Float) (Variables|Default|GetPotentialLife)))))

(fn ModifyHealth
  (params (Modification :type Float%20%28double-precision%29))
  (bind _stats (CallFunction|CurrentStats))
  (if (> (+ (Variables|Default|GetHealth) Modification) (.maxhealth _stats))
    (Variables|Default|SetHealth (.maxhealth _stats))
    (switch Utilities|FlowControl|Switch|SwitchonE_State (Variables|Default|GetCurrentState) :!label _label
      (:NewEnumerator0
        (if (< (Variables|Default|GetHealth) (Variables|Default|GetUndeadThreshold))
          (CallFunction|ChangeState "NewEnumerator1")))
      (:NewEnumerator1
        (if (> (Variables|Default|GetHealth) (Variables|Default|GetUndeadThreshold))
          (CallFunction|ChangeState "NewEnumerator0"))))
    (elif (< (+ (Variables|Default|GetHealth) Modification) (.minhealth _stats))
      (Variables|Default|SetHealth (.minhealth _stats))
      (CallFunction|Die)
      (else
        (Variables|Default|SetHealth (+ (Variables|Default|GetHealth) Modification))
        (goto _label))))
  (Development|PrintString (Utilities|String|Append "Current health : " (Utilities|String|ToString(Float) (Variables|Default|GetHealth)))))

(fn ChangeState
  (params (NewState :type E_State%20Enum :default "NewEnumerator0"))
  (bind _statevfx (Variables|Default|GetStateVFX))
  (bind _output_get (Variables|Default|SetCurrentState NewState))
  (switch Utilities|FlowControl|Switch|SwitchonE_State _output_get
    (:NewEnumerator0
      (Sprite|SetFlipbook _statevfx "/Game/Game/VFX/AliveVFX/FB_AliveVFX.FB_AliveVFX"))
    (:NewEnumerator1
      (Sprite|SetFlipbook _statevfx "/Game/Game/VFX/UndeadVFX/FB_UndeadVFX.FB_UndeadVFX"))))

(fn Die
  (bind _asplayer_controller (Utilities|Casting|CastToPlayerController (Pawn|GetController)))
  (Default|CallOnPlayerDeath (Class|GameplayStatics|GetPlayerControllerID _asplayer_controller)))

(fn PaySpecial
  (bind _stats (CallFunction|CurrentStats))
  (bind _returnvalue (* (.specialcost _stats) -1.0))
  (switch Utilities|FlowControl|Switch|SwitchonE_State (Variables|Default|GetCurrentState)
    (:NewEnumerator0
      (if (> (- (Variables|Default|GetHealth) (.minhealth _stats)) (.specialcost _stats))
        (CallFunction|ModifyHealth _returnvalue)
        (else
          (return false))))
    (:NewEnumerator1
      (if (>= (Variables|Default|GetPotentialLife) (.specialcost _stats))
        (CallFunction|ModifyPotentialLife _returnvalue)
        (else
          (return false)))))
  (return true))

(fn LoadStatsfromGameInstance
  (bind _asbp_game_instance (Utilities|Casting|CastToBP_GameInstance (Game|GetGameInstance)))
  (bind _asplayer_controller (Utilities|Casting|CastToPlayerController (Pawn|GetController)))
  (if (.ReturnValue (Utilities|Map|Find (Variables|/Game/Game/GameSettings/BP_GameInstance.BP_GameInstance_C|GetSavedBoons _asbp_game_instance) (Class|GameplayStatics|GetPlayerControllerID _asplayer_controller)))
    (for _array_element (.boons (.Value (Utilities|Map|Find (Variables|/Game/Game/GameSettings/BP_GameInstance.BP_GameInstance_C|GetSavedBoons _asbp_game_instance) (Class|GameplayStatics|GetPlayerControllerID _asplayer_controller))))
      (bind _returnvalue (Game|ConstructObjectfromClass _array_element))
      (CallFunction|ModifyStat (Variables|/Game/Game/Boons/BP_BaseBoon.BP_BaseBoon_C|GetModifier _returnvalue)))
    (Variables|Default|SetHealth (.health (.Value (Utilities|Map|Find (Variables|/Game/Game/GameSettings/BP_GameInstance.BP_GameInstance_C|GetSavedRessources _asbp_game_instance) (Class|GameplayStatics|GetPlayerControllerID _asplayer_controller)))))
    (Variables|Default|SetPotentialLife (.potentiallife (.Value (Utilities|Map|Find (Variables|/Game/Game/GameSettings/BP_GameInstance.BP_GameInstance_C|GetSavedRessources _asbp_game_instance) (Class|GameplayStatics|GetPlayerControllerID _asplayer_controller)))))
    (CallFunction|ModifyHealth 0.0)))